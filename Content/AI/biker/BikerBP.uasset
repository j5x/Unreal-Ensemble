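; BikerBP is an AI biker pawn that wanders the navmesh, alternating between roaming and idling.
; Tick branches on IsIdle: when false, it waits a random delay, then uses AIMoveTo toward a random reachable point nearby.
; A successful move sets IsIdle, so the mesh plays a breathing idle animation between short delays before roaming resumes.
; Latent Delays inside Tick pace the loop, with no behavior tree.
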(event EventBeginPlay)

(event Collision|EventActorBeginOverlap
  (params (OtherActor :type Actor%20Object%20Reference)))

(event EventTick
  (params (DeltaSeconds :type Float%20%28single-precision%29))
  (Utilities|FlowControl|Sequence
    (:then_0
      (if (not (Variables|Default|GetisIdle))
        (Utilities|FlowControl|Delay (Math|Random|RandomFloatinRange 1.5 3.0))
        (AI|AIMoveTo self (.RandomLocation (AI|Navigation|GetRandomReachablePointinRadius (Transformation|GetActorLocation) 1e+03 0 "/Script/NavigationSystem.RecastFilter_UseDefaultArea")) 0 5.0 false
          (:OnSuccess
            (Variables|Default|SetisIdle true)))
        (else
          (Utilities|FlowControl|Delay 0.5)
          (Components|Animation|SetAnimation (Variables|Character|GetMesh) "/Game/AI/Animations/Breathing_Idle_Biker.Breathing_Idle_Biker")
          (Utilities|FlowControl|Delay 1.5)
          (Variables|Default|SetisIdle false))))))

(fn ConstructionScript)